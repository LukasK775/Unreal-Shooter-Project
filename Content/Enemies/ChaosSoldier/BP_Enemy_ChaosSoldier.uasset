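; Chaos Soldier enemy character that handles taking damage and dying.
; Non-lethal hits report an AI damage sense event, always crediting the player, and play a hurt sound.
; At zero health it flags Dead on the blackboard, notifies its AI controller, plays the death animation and disables collision.
; It then drops a small bullet pickup, adds a kill to the game instance and plays a death sound.
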(event `self.ReceiveBeginPlay`)

(event `self.ReceiveAnyDamage`
  (params (Damage :type "Float (single-precision)") (DamageType :type "DamageType Object Reference") (InstigatedBy :type "Controller Object Reference") (DamageCauser :type "Actor Object Reference"))
  (bind _output_get (set `self.Health` (- (`self.Health`) Damage)))
  (if (> _output_get 0.0)
    (`AISense_Damage.ReportDamageEvent` self (`GameplayStatics.GetPlayerCharacter` 0))
    (`GameplayStatics.SpawnSoundAtLocation` "/Game/Sounds/Enemies/chaosenemy_hurt.chaosenemy_hurt" (`self.K2_GetActorLocation`) (struct) 0.3 1.0 0.0 "/Game/Sounds/SoundAttenGeneric.SoundAttenGeneric" null)
    (else
      (bind _asai_chaos_soldier (cast `/Game/Enemies/ChaosSoldier/AI_ChaosSoldier` (`self.GetController`)))
      (`BlackboardComponent.SetValueAsBool` (`AIBlueprintHelperLibrary.GetBlackboard` _asai_chaos_soldier) "Dead" true)
      (`/Game/Enemies/ChaosSoldier/AI_ChaosSoldier.Killed` _asai_chaos_soldier)
      (`SkeletalMeshComponent.PlayAnimation` (`self.Mesh`) "/Game/EnemyContent/ChaosSoldier/die.die" false)
      (`PrimitiveComponent.SetCollisionEnabled` (`self.CapsuleComponent`) "NoCollision")
      (`PrimitiveComponent.SetCollisionEnabled` (`self.Mesh`) "NoCollision")
      (bind _returnvalue (`|SpawnActorFromClass` "/Game/Pickups/Pickup_Bullets_Small.Pickup_Bullets_Small_C" (`self.GetTransform`) "Undefined" "MultiplyWithRoot" null null))
      (set `/Game/Pickups/Pickup_Bullets_Small.BaseAmmo` 5 _returnvalue)
      (bind _asbp_first_person_game_instance (cast `/Game/FirstPerson/Blueprints/BP_FirstPersonGameInstance` (`GameplayStatics.GetGameInstance`)))
      (`/Game/FirstPerson/Blueprints/BP_FirstPersonGameInstance.AddKill` _asbp_first_person_game_instance)
      (`GameplayStatics.PlaySoundAtLocation` "/Game/Sounds/Enemies/chaosenemy_die.chaosenemy_die" (`self.K2_GetActorLocation`) (struct) 0.3 1.0 0.0 "/Game/Sounds/SoundAttenGeneric.SoundAttenGeneric" null null null))))

(fn `UserConstructionScript`)