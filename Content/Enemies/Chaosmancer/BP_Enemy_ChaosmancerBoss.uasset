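; Chaosmancer boss enemy Blueprint that handles taking damage and dying, with movement and attacks not defined here.
; Non-projectile damage lowers Health; while alive it reports a damage event with the player as instigator and plays a hurt sound.
; Death flags the blackboard, notifies AI_Chaosmancer, plays the death animation and sound, and disables collision.
; It also records a kill on the GameInstance and sends TagOpenOnDeath to the GameMode as a player-caused interaction.
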(event `self.ReceiveBeginPlay`)

(event `self.ReceiveAnyDamage`
  (params (Damage :type "Float (single-precision)") (DamageType :type "DamageType Object Reference") (InstigatedBy :type "Controller Object Reference") (DamageCauser :type "Actor Object Reference"))
  (if (!= DamageType "/Game/DamageTypes/DamageType_Projectile.DamageType_Projectile")
    (bind _output_get (set `self.Health` (- (`self.Health`) Damage)))
    (if (> _output_get 0.0)
      (`AISense_Damage.ReportDamageEvent` self (`GameplayStatics.GetPlayerCharacter` 0))
      (`GameplayStatics.PlaySoundAtLocation` "/Game/Sounds/Enemies/chaoselemental_hurt.chaoselemental_hurt" (`self.K2_GetActorLocation`) (struct) 0.3 1.0 0.0 "/Game/Sounds/SoundAttenGeneric.SoundAttenGeneric" null null null)
      (else
        (bind _asai_chaosmancer (cast `/Game/Enemies/Chaosmancer/AI_Chaosmancer` (`self.GetController`)))
        (`BlackboardComponent.SetValueAsBool` (`AIBlueprintHelperLibrary.GetBlackboard` null) "Dead" true)
        (`/Game/Enemies/Chaosmancer/AI_Chaosmancer.Killed` _asai_chaosmancer)
        (`SkeletalMeshComponent.PlayAnimation` (`self.Mesh`) "/Game/EnemyContent/Chaosmancer/die.die" false)
        (`PrimitiveComponent.SetCollisionEnabled` (`self.CapsuleComponent`) "NoCollision")
        (`PrimitiveComponent.SetCollisionEnabled` (`self.Mesh`) "NoCollision")
        (bind _asbp_first_person_game_instance (cast `/Game/FirstPerson/Blueprints/BP_FirstPersonGameInstance` (`GameplayStatics.GetGameInstance`)))
        (`/Game/FirstPerson/Blueprints/BP_FirstPersonGameInstance.AddKill` _asbp_first_person_game_instance)
        (`GameplayStatics.PlaySoundAtLocation` "/Game/Sounds/Enemies/chaoselemental_die.chaoselemental_die" (`self.K2_GetActorLocation`) (struct) 0.6 0.5 0.0 "/Game/Sounds/SoundAttenGeneric.SoundAttenGeneric" null null null)
        (bind _asbp_first_person_game_mode (cast `/Game/FirstPerson/Blueprints/BP_FirstPersonGameMode` (`GameplayStatics.GetGameMode`)))
        (`/Game/FirstPerson/Blueprints/BP_FirstPersonGameMode.PlayerCauseInteraction` _asbp_first_person_game_mode (`self.TagOpenOnDeath`))))))

(fn `UserConstructionScript`)