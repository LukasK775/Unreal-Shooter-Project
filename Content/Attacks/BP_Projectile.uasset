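; Shared projectile for plasma, grenade, rocket and Chaos enemy attacks, with ProjType selecting its behaviour.
; ProjectileInit sets mesh, light and pulse animation per type, applies speed and bounce from lookup maps, and ignores creator collision.
; Hits destroy it, spawn type-specific effects, then apply direct damage or, for types with a radius, radial damage plus character knockback.
; Mega Plasma Bolts periodically trace random directions to draw cosmetic Niagara lightning to nearby surfaces.
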(event `self.ReceiveTick`
  (params (DeltaSeconds :type "Float (single-precision)"))
  (bind _returnvalue (`self.K2_GetActorLocation`))
  (if (not (`|EnumInequality` (`self.ProjType`) "NewEnumerator2"))
    (set `self.ProjectileTimer` (+ DeltaSeconds (`self.ProjectileTimer`)))
    (if (>= (`self.ProjectileTimer`) 0.25)
      (set `self.ProjectileTimer` 0.0)
      (for _ (range (+ (`KismetMathLibrary.RandomIntegerInRange` 6 12) 1))
        (set `self.RandDir` (`KismetMathLibrary.RandomUnitVector`))
        (bind _outhit (`KismetSystemLibrary.LineTraceSingle` (+ _returnvalue (* (`self.RandDir`) 1.0)) (+ _returnvalue (* (`self.RandDir`) 700.0)) "TraceTypeQuery1"))
        (bind (_bblockinghit _binitialoverlap _time _distance _location _impactpoint) (`GameplayStatics.BreakHitResult` _outhit))
        (if _bblockinghit
          (bind _returnvalue_2 (`NiagaraFunctionLibrary.SpawnSystemAttached` "/Game/Effects/IonCannonLightning.IonCannonLightning" (`self.ProjectileMesh`) "Electric" (0.0 0.0 0.0) (struct) "KeepWorldPosition" true))
          (`NiagaraComponent.SetVariableVec3` _returnvalue_2 "BeamStart" (`self.K2_GetActorLocation`))
          (`NiagaraComponent.SetVariableVec3` _returnvalue_2 "BeamEnd" _impactpoint))))))

(event `ProjectileInit`
  (`self.SetProjectileModel`)
  (`self.SetProjectileStats`)
  (`PrimitiveComponent.IgnoreActorWhenMoving` (`self.Collider`) (`self.Creator`) true)
  (bind _asbp_first_person_character (cast `/Game/FirstPerson/Blueprints/BP_FirstPersonCharacter` (`self.Creator`))
    (:`then`
      (`PrimitiveComponent.IgnoreActorWhenMoving` (`Character.CapsuleComponent` _asbp_first_person_character) self true))
    (:`CastFailed`
      _))
  (set `self.Initialised` true))

(event `self.Collider.OnComponentHit`
  (params (HitComponent :type "PrimitiveComponent Object Reference") (OtherActor :type "Actor Object Reference") (OtherComp :type "PrimitiveComponent Object Reference") (NormalImpulse :type "Vector Structure") (Hit :type "HitResult Structure (by ref)"))
  (bind (_bblockinghit _binitialoverlap _time _distance _location _impactpoint _normal _impactnormal _physmat _hitactor) (`GameplayStatics.BreakHitResult` Hit))
  (bind (_value _returnvalue) (`BlueprintMapLibrary.Map_Find` (`self.ProjectileRadius`) (`self.ProjType`)))
  (bind _returnvalue_2 (`KismetMathLibrary.Conv_IntToDouble` (`BlueprintMapLibrary.Map_Find` (`self.ProjectileDamageStats`) (`self.ProjType`))))
  (if (`self.Initialised`)
    (if (or (!= _hitactor (`self.Creator`)) (and (== _hitactor (`self.Creator`)) (`BlueprintMapLibrary.Map_Find` (`self.ProjectileCanHitCreator`) (`self.ProjType`))))
      (if (not (== OtherActor (`self.Creator`)))
        (`self.K2_DestroyActor`)
        (`self.ExplodeEffect` _impactpoint)
        (if _returnvalue
          (`GameplayStatics.ApplyRadialDamage` :`BaseDamage` _returnvalue_2 :`Origin` _impactpoint :`DamageRadius` _value :`DamageTypeClass` "/Game/DamageTypes/DamageType_Projectile.DamageType_Projectile_C" :`DamageCauser` null :`InstigatedByController` null)
          (bind _outactors (`GameplayStatics.GetAllActorsOfClass` "/Script/Engine.Character"))
          (for _array_element _outactors
            (bind _returnvalue_3 (`self.K2_GetActorLocation` _array_element))
            (if (<= (`KismetMathLibrary.Vector_Distance` _impactpoint _returnvalue_3) _value)
              (bind _ascharacter (cast `Character` _array_element))
              (`Character.LaunchCharacter` _ascharacter (* (`KismetMathLibrary.GetDirectionUnitVector` _impactpoint _returnvalue_3) (* _returnvalue_2 5.0)) false false)))
          (else
            (`GameplayStatics.ApplyDamage` _hitactor _returnvalue_2)))))))

(event `PlasmaBoltAnimation`
  (bind (_direction _scaletrack) (`Timeline|PlasmaTimescale`)
    (:`Update`
      (`SceneComponent.SetRelativeScale3D` (`self.ProjectileMesh`) (`KismetMathLibrary.Conv_DoubleToVector` (* _scaletrack 0.5))))))

(fn `ExplodeEffect`
  (params (Location :type "Vector Structure"))
  (switch `/Game/Enums/ProjectileTypeEnum` (`self.ProjType`)
    (:`NewEnumerator1`
      (`NiagaraFunctionLibrary.SpawnSystemAtLocation` "/Game/Effects/PlasmaHit.PlasmaHit" Location)
      (`GameplayStatics.PlaySoundAtLocation` "/Game/Sounds/Weapons/plasmahit.plasmahit" Location (struct) 0.6 (`KismetMathLibrary.RandomFloatInRange` 0.8 1.2) 0.0 "/Game/Sounds/SoundAttenGeneric.SoundAttenGeneric" null null null))
    (:`NewEnumerator2`
      (`NiagaraFunctionLibrary.SpawnSystemAtLocation` "/Game/Effects/IonCannonHit.IonCannonHit" Location)
      (`GameplayStatics.PlaySoundAtLocation` "/Game/Sounds/Weapons/ioncannonexplode.ioncannonexplode" Location (struct) 1.0 1.0 0.0 "/Game/Sounds/SoundAttenGeneric.SoundAttenGeneric" null null null))
    (:`NewEnumerator5`
      (`NiagaraFunctionLibrary.SpawnSystemAtLocation` "/Game/Effects/HauntedHit.HauntedHit" Location))
    (:`NewEnumerator6`
      (`NiagaraFunctionLibrary.SpawnSystemAtLocation` "/Game/Effects/ChaosmancerWeakHit.ChaosmancerWeakHit" Location)
      (`GameplayStatics.PlaySoundAtLocation` "/Game/Sounds/Weapons/plasmahit.plasmahit" Location (struct) 0.6 (`KismetMathLibrary.RandomFloatInRange` 0.8 1.2) 0.0 "/Game/Sounds/SoundAttenGeneric.SoundAttenGeneric" null null null))
    (:`NewEnumerator7`
      (`NiagaraFunctionLibrary.SpawnSystemAtLocation` "/Game/Effects/ChaosmancerStrongHit.ChaosmancerStrongHit" Location)
      (`GameplayStatics.PlaySoundAtLocation` "/Game/Sounds/Weapons/ioncannonexplode.ioncannonexplode" Location (struct) 1.0 1.0 0.0 "/Game/Sounds/SoundAttenGeneric.SoundAttenGeneric" null null null))))

(fn `SetProjectileModel`
  (bind _projectilemesh (`self.ProjectileMesh`))
  (bind _pointlight (`self.PointLight`))
  (switch `/Game/Enums/ProjectileTypeEnum` (`self.ProjType`)
    (:`NewEnumerator1`
      (`StaticMeshComponent.SetStaticMesh` _projectilemesh "/Game/Attacks/ProjectilePlasmaBolt.ProjectilePlasmaBolt")
      (`self.PlasmaBoltAnimation`))
    (:`NewEnumerator2`
      (`StaticMeshComponent.SetStaticMesh` _projectilemesh "/Game/Attacks/ProjectileMegaPlasmaBolt.ProjectileMegaPlasmaBolt")
      (`self.PlasmaBoltAnimation`)
      (`LightComponent.SetLightColor` _pointlight (struct :`R` 0.114558 :`G` 1.0 :`A` 1.0) true)
      (`LightComponent.SetIntensity` _pointlight 10000.0))
    (:`NewEnumerator3`
      (`StaticMeshComponent.SetStaticMesh` _projectilemesh "/Game/Attacks/ProjectileGrenade.ProjectileGrenade"))
    (:`NewEnumerator4`
      (`StaticMeshComponent.SetStaticMesh` _projectilemesh "/Game/Attacks/ProjectileRocket.ProjectileRocket"))
    (:`NewEnumerator5`
      (`StaticMeshComponent.SetStaticMesh` _projectilemesh "/Game/Attacks/ProjectileChaosBolt.ProjectileChaosBolt")
      (`self.PlasmaBoltAnimation`)
      (`LightComponent.SetLightColor` (`self.PointLight`) (struct :`R` 1.0 :`G` 0.16251 :`B` 0.24222 :`A` 1.0) true))
    (:`NewEnumerator6`
      (`StaticMeshComponent.SetStaticMesh` _projectilemesh "/Game/Attacks/ProjectileChaosmancerWeak.ProjectileChaosmancerWeak")
      (`self.PlasmaBoltAnimation`)
      (`LightComponent.SetLightColor` (`self.PointLight`) (struct :`G` 1.0 :`B` 0.553934 :`A` 1.0) true))
    (:`NewEnumerator7`
      (`StaticMeshComponent.SetStaticMesh` _projectilemesh "/Game/Attacks/ProjectileChaosmancerStrong.ProjectileChaosmancerStrong")
      (`self.PlasmaBoltAnimation`)
      (`LightComponent.SetLightColor` (`self.PointLight`) (struct :`R` 1.0 :`B` 0.211852 :`A` 1.0) true))))

(fn `SetProjectileStats`
  (bind _projtype (`self.ProjType`))
  (bind _projectilemover (`self.ProjectileMover`))
  (bind _output_get (set `ProjectileMovementComponent.InitialSpeed` (`BlueprintMapLibrary.Map_Find` (`self.ProjectileSpeedStats`) _projtype) _projectilemover))
  (set `MovementComponent.Velocity` (* _output_get (`MovementComponent.Velocity` _projectilemover)) _projectilemover)
  (set `ProjectileMovementComponent.bShouldBounce` (`BlueprintMapLibrary.Map_Find` (`self.ProjectileBounces`) _projtype) _projectilemover))

(fn `UserConstructionScript`)